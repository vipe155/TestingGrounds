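; Demon enemy character that handles its health, death animation and dissolve effect.
; BeginPlay creates dynamic material instances for the mesh's four material slots.
; AnyDamage subtracts from Health and, once it reaches zero or below, plays the death animation and a timeline that drives DissolveAmount on those materials.
; The controller is unpossessed from the timeline's update, so that call repeats throughout the dissolve; KillCharacter is not called here and TakeDamage is empty.
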(event EventTick
  (params (DeltaSeconds :type Float%20%28single-precision%29)))

(event Game|Damage|EventAnyDamage
  (params (Damage :type Float%20%28single-precision%29) (DamageType :type Damage%20Type%20Object%20Reference) (InstigatedBy :type Controller%20Object%20Reference) (DamageCauser :type Actor%20Object%20Reference))
  (Variables|Default|SetHealth (- (Variables|Default|GetHealth) Damage))
  (if (CallFunction|IsDead)
    (Components|Animation|PlayAnimation (Variables|Character|GetMesh) "/Game/Demon/MeshAndAnimations/Demon4/Demon_Anim_metarig_Death.Demon_Anim_metarig_Death" false)
    (bind _dissolve (Timeline|DissolveTimeline Play)
      (:Update
        (Rendering|Material|SetScalarParameterValue (Variables|Default|GetDissolveMaterial) "DissolveAmount" _dissolve :!class /Script/Engine.MaterialInstanceDynamic)
        (Pawn|UnPossess (Pawn|GetController))))))

(event EventBeginPlay
  (CallFunction|SetDemonMaterial))

(fn ConstructionScript)

(fn IsDead
  (return (<= (Variables|Default|GetHealth) 0.0)))

(fn KillCharacter
  (Pawn|UnPossess (Pawn|GetController)))

(fn TakeDamage
  (params (Health :type Float%20%28single-precision%29)))

(fn SetDemonMaterial
  (bind _mesh (Variables|Character|GetMesh))
  (bind _mesh_2 (Variables|Character|GetMesh))
  (bind _mesh_3 (Variables|Character|GetMesh))
  (bind _returnvalue (Rendering|Material|CreateDynamicMaterialInstance (Variables|Character|GetMesh) 0 (Rendering|Material|GetMaterial (Variables|Character|GetMesh) 0) :!class /Script/Engine.PrimitiveComponent))
  (Variables|Default|SetDissolveMaterial _returnvalue)
  (bind _returnvalue_2 (Rendering|Material|CreateDynamicMaterialInstance _mesh 1 (Rendering|Material|GetMaterial _mesh 1) :!class /Script/Engine.PrimitiveComponent))
  (Variables|Default|SetDissolveMaterial1 _returnvalue_2)
  (bind _returnvalue_3 (Rendering|Material|CreateDynamicMaterialInstance _mesh_3 2 (Rendering|Material|GetMaterial _mesh_3 2) :!class /Script/Engine.PrimitiveComponent))
  (Variables|Default|SetDissolveMaterial2 _returnvalue_3)
  (bind _returnvalue_4 (Rendering|Material|CreateDynamicMaterialInstance _mesh_2 3 (Rendering|Material|GetMaterial _mesh_2 3) :!class /Script/Engine.PrimitiveComponent))
  (Variables|Default|SetDissolveMaterial3 _returnvalue_4))