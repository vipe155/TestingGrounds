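; Demon enemy character that chases Characters it sees and dissolves when its health runs out.
; PawnSensing drives a repeating AIMoveTo, with retriggerable delays clearing the seen flag after sight lapses.
; DoOnce gates switch between chase speed and a timeline-eased slowdown on an attack trigger, while Tick sets an unseen walk speed; random roaming is unconnected.
; Lethal damage animates dissolve on four dynamic mesh materials and unpossesses the controller.
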(event OnSeePawn(PawnSensing)
  (params (Pawn :type Pawn%20Object%20Reference))
  (bind _charactermovement (Variables|Character|GetCharacterMovement))
  (Utilities|FlowControl|Sequence
    (:then_0
      (Variables|Default|SetPlayer%20Is%20BEING%20Seen true)
      (Variables|Default|SetPlayer%20Has%20Been%20Seen true)
      (bind _ascharacter (Utilities|Casting|CastToCharacter Pawn :!label _label))
      (AI|AIMoveTo self "0, 0, 0" _ascharacter 1.5e+02 false
        (:then
          (if (Variables|Default|GetPlayer%20Has%20Been%20Seen)
            (Utilities|FlowControl|RetriggerableDelay 1.0)
            (goto _label)))))
    (:then_1
      (if (Variables|Default|GetAttack%20Slow%20Down%20Trigger)
        (Utilities|FlowControl|DoOnce false :!label _label_2
          (:Completed
            (bind _lerp_value (Timeline|Speed%20Slow%20Down%20Timeline PlayFromStart)
              (:Update
                (Variables|/Script/Engine.CharacterMovementComponent|SetMaxWalkSpeed _charactermovement (Math|Float|Lerp 5e+02 7e+01 _lerp_value))
                (Variables|/Script/Engine.CharacterMovementComponent|SetMaxAcceleration _charactermovement (Math|Float|Lerp 3e+02 1e+02 _lerp_value))
                (goto _label_3 Reset)))))
        (else
          (Utilities|FlowControl|DoOnce false :!label _label_3
            (:Completed
              (Variables|/Script/Engine.CharacterMovementComponent|SetMaxWalkSpeed _charactermovement 5e+02)
              (Variables|/Script/Engine.CharacterMovementComponent|SetMaxAcceleration _charactermovement 4e+02)
              (goto _label_2 Reset))))))
    (:then_2
      (Utilities|FlowControl|RetriggerableDelay 4.0)
      (Variables|Default|SetPlayer%20Has%20Been%20Seen false))))

(event Game|Damage|EventAnyDamage
  (params (Damage :type Float%20%28single-precision%29) (DamageType :type Damage%20Type%20Object%20Reference) (InstigatedBy :type Controller%20Object%20Reference) (DamageCauser :type Actor%20Object%20Reference))
  (Variables|Default|SetHealth (- (Variables|Default|GetHealth) Damage))
  (if (CallFunction|IsDead)
    (bind _dissolve (Timeline|DissolveTimeline Play)
      (:Update
        (Rendering|Material|SetScalarParameterValue (Variables|Default|GetDissolveMaterial) "DissolveAmount" _dissolve :!class /Script/Engine.MaterialInstanceDynamic)
        (CallFunction|KillCharacter)))))

(event EventBeginPlay
  (CallFunction|SetDemonMaterial))

(event EventTick
  (params (DeltaSeconds :type Float%20%28single-precision%29))
  (bind _charactermovement (Variables|Character|GetCharacterMovement))
  (bind _charactermovement_2 (Variables|Character|GetCharacterMovement))
  (if (not (Variables|Default|GetPlayer%20Has%20Been%20Seen))
    (Utilities|FlowControl|DoOnce false
      (:Completed
        (Variables|/Script/Engine.CharacterMovementComponent|SetMaxWalkSpeed _charactermovement 1e+02)
        (Variables|/Script/Engine.CharacterMovementComponent|SetMaxAcceleration _charactermovement 5e+01)
        (Utilities|FlowControl|Sequence
          (:then_0
            (Utilities|FlowControl|DoOnce false) ; enters at Reset
          )
          (:then_1
            (Utilities|FlowControl|DoOnce false) ; enters at Reset
          ))))))

(fn ConstructionScript)

(fn IsDead
  (return (<= (Variables|Default|GetHealth) 0.0)))

(fn KillCharacter
  (Pawn|UnPossess (Pawn|GetController)))

(fn TakeDamage
  (params (Health :type Float%20%28single-precision%29)))

(fn SetDemonMaterial
  (bind _mesh (Variables|Character|GetMesh))
  (bind _mesh_2 (Variables|Character|GetMesh))
  (bind _mesh_3 (Variables|Character|GetMesh))
  (bind _returnvalue (Rendering|Material|CreateDynamicMaterialInstance (Variables|Character|GetMesh) 0 (Rendering|Material|GetMaterial (Variables|Character|GetMesh) 0) :!class /Script/Engine.PrimitiveComponent))
  (Variables|Default|SetDissolveMaterial _returnvalue)
  (bind _returnvalue_2 (Rendering|Material|CreateDynamicMaterialInstance _mesh 1 (Rendering|Material|GetMaterial _mesh 1) :!class /Script/Engine.PrimitiveComponent))
  (Variables|Default|SetDissolveMaterial1 _returnvalue_2)
  (bind _returnvalue_3 (Rendering|Material|CreateDynamicMaterialInstance _mesh_3 2 (Rendering|Material|GetMaterial _mesh_3 2) :!class /Script/Engine.PrimitiveComponent))
  (Variables|Default|SetDissolveMaterial2 _returnvalue_3)
  (bind _returnvalue_4 (Rendering|Material|CreateDynamicMaterialInstance _mesh_2 3 (Rendering|Material|GetMaterial _mesh_2 3) :!class /Script/Engine.PrimitiveComponent))
  (Variables|Default|SetDissolveMaterial3 _returnvalue_4))